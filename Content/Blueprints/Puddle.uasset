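; Puddle actor tagged "Water" that grows in, lingers for a set time, then shrinks away and destroys itself.
; The construction script stores the placed scale as the maximum and collapses the actor to near zero.
; Tick runs a three-phase timer using Stay and Fade flags, scaling linearly over the fade-in and fade-out durations.
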(event `self.ReceiveTick`
  (params (DeltaSeconds :type "Float (single-precision)"))
  (set `self.Elapsed` (+ DeltaSeconds (`self.Elapsed`)))
  (if (`self.Fade`)
    (`self.SetActorScale3D` (- (`self.GetActorScale3D`) (* (/ (`self.MaxScale`) (`self.FadeOutDuration`)) DeltaSeconds)))
    (if (>= (`self.Elapsed`) (`self.FadeOutDuration`))
      (`self.K2_DestroyActor`))
    (elif (`self.Stay`)
      (if (>= (`self.Elapsed`) (`self.StayDuration`))
        (set `self.Fade` true)
        (set `self.Elapsed` 0.0))
      (else
        (`self.SetActorScale3D` (+ (`self.GetActorScale3D`) (* (/ (`self.MaxScale`) (`self.FadeInDuration`)) DeltaSeconds)))
        (if (>= (`self.Elapsed`) (`self.FadeInDuration`))
          (set `self.Stay` true)
          (set `self.Elapsed` 0.0))))))

(fn `UserConstructionScript`
  (set `self.Tags` (`|MakeArray` "Water" :!type "Name"))
  (set `self.MaxScale` (`self.GetActorScale3D`))
  (`self.SetActorScale3D` (0.001 0.001 0.001)))