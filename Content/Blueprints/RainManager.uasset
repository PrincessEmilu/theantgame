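; RainManager is an actor that produces rain by continually spawning Raindrop actors around its own location.
; Tick accumulates elapsed time and spawns a drop once the current interval passes, then picks the next interval randomly around an average with a set variation.
; SpawnRaindrop places each drop at a random point within a box defined by SpawnRange, centered on the actor.
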(event `self.ReceiveTick`
  (params (DeltaSeconds :type "Float (single-precision)"))
  (bind _avgtimebetween_drops (`self.AvgTimeBetween Drops`))
  (bind _timevariation (`self.TimeVariation`))
  (bind _output_get (set `self.TimeSinceLastDrop` (+ DeltaSeconds (`self.TimeSinceLastDrop`))))
  (if (>= _output_get (`self.TimeToNextDrop`))
    (`self.Spawn Raindrop`)
    (set `self.TimeSinceLastDrop` 0.0)
    (set `self.TimeToNextDrop` (`KismetMathLibrary.RandomFloatInRange` (- _avgtimebetween_drops _timevariation) (+ _avgtimebetween_drops _timevariation)))))

(fn `Spawn Raindrop`
  (bind _x (.x (`self.K2_GetActorLocation`)))
  (bind _y (.y (`self.K2_GetActorLocation`)))
  (bind _z (.z (`self.K2_GetActorLocation`)))
  (bind _x_2 (.x (`self.SpawnRange`)))
  (bind _y_2 (.y (`self.SpawnRange`)))
  (bind _z_2 (.z (`self.SpawnRange`)))
  (`|SpawnActorFromClass` "/Game/Blueprints/Raindrop.Raindrop_C" (`KismetMathLibrary.MakeTransform` (`KismetMathLibrary.MakeVector` (`KismetMathLibrary.RandomFloatInRange` (- _x _x_2) (+ _x _x_2)) (`KismetMathLibrary.RandomFloatInRange` (- _y _y_2) (+ _y _y_2)) (`KismetMathLibrary.RandomFloatInRange` (- _z _z_2) (+ _z _z_2)))) "Undefined" "OverrideRootScale" null null))

(fn `UserConstructionScript`)