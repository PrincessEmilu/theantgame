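; Raindrop actor that falls straight down via ProjectileMovement and leaves puddles where it lands.
; The construction script tags it Water and sets its downward velocity, so overlaps with other Water-tagged actors are ignored.
; Any other overlap destroys the drop, first spawning a Puddle unless the other actor is tagged Shelter or Player.
; A short downward visibility trace supplies the distance used to lower the puddle onto the surface below.
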(event `self.ReceiveActorBeginOverlap`
  (params (OtherActor :type "Actor Object Reference"))
  (bind _returnvalue (`self.K2_GetActorLocation`))
  (if (not (`self.ActorHasTag` OtherActor "Water"))
    (if (not (or (`self.ActorHasTag` OtherActor "Shelter") (`self.ActorHasTag` OtherActor "Player")))
      (bind _outhit (`KismetSystemLibrary.LineTraceSingle` _returnvalue (+ _returnvalue (* (`KismetMathLibrary.GetUpVector` (struct)) -100.0)) "TraceTypeQuery1"))
      (bind (_bblockinghit _binitialoverlap _time _distance _location _impactpoint _normal _impactnormal _physmat _hitactor) (`GameplayStatics.BreakHitResult` _outhit))
      (if (`KismetSystemLibrary.IsValid` _hitactor)
        (set `self.Distance` _distance))
      (`|SpawnActorFromClass` "/Game/Blueprints/Puddle.Puddle_C" (`KismetMathLibrary.MakeTransform` (`KismetMathLibrary.MakeVector` (.x (`self.K2_GetActorLocation`)) (.y (`self.K2_GetActorLocation`)) (- (.z (`self.K2_GetActorLocation`)) (`self.Distance`)))) "AlwaysSpawn" "OverrideRootScale" null null))
    (`self.K2_DestroyActor`)))

(event `self.ReceiveTick`
  (params (DeltaSeconds :type "Float (single-precision)")))

(fn `UserConstructionScript`
  (set `self.Tags` (`|MakeArray` "Water" :!type "Name"))
  (set `MovementComponent.Velocity` (0.0 0.0 -1500.0) (`self.ProjectileMovement`)))